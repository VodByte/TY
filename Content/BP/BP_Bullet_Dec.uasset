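; BP_Bullet_Dec is a bullet actor that damages whatever its collision sphere begins to overlap, then destroys itself.
; On BeginPlay it sets a lifespan from a variable so it expires on its own.
; On overlap it applies base damage with its owner as causer, and an enemy character hit also plays the first player's HUD hit animation before destruction.
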(event OnComponentBeginOverlap(SphereCollision)
  (params (OverlappedComponent :type Primitive%20Component%20Object%20Reference) (OtherActor :type Actor%20Object%20Reference) (OtherComp :type Primitive%20Component%20Object%20Reference) (OtherBodyIndex :type Integer) (bFromSweep :type Boolean) (SweepResult :type Hit%20Result%20Structure%20%28by%20ref%29))
  (Game|Damage|ApplyDamage OtherActor (Variables|Default|GetBaseDamage) 0 (Components|GetOwner))
  (Utilities|Casting|CastToBP_Character_Enemy OtherActor
    (:then
      (bind _ashud_ty (Utilities|Casting|CastToHUD_TY (HUD|GetHUD (Game|GetPlayerController 0))))
      (Default|PlayHittedAnim _ashud_ty))
    (:CastFailed
      _))
  (Actor|DestroyActor))

(event EventBeginPlay
  (Actor|SetLifeSpan (Variables|Default|GetLifeSpan)))

(event Collision|EventActorBeginOverlap
  (params (OtherActor :type Actor%20Object%20Reference)))

(event EventTick
  (params (DeltaSeconds :type Float%20%28single-precision%29)))

(fn ConstructionScript)