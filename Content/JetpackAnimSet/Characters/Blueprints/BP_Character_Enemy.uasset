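; Jetpack enemy character that starts its jetpack on spawn and is driven by an AI controller.
; AI Perception sets the CanChasePlayer blackboard bool whenever it gains or loses sight or sense of a BP_Character_Master.
; SetActorFunction toggles brain logic, perception, collision and tick together, called on melee damage and zero HP.
; Melee kills switch to falling after a strike-animation delay; other deaths explode and destroy the actor.
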(event OnTargetPerceptionUpdated(AIPerception)
  (params (Actor :type Actor%20Object%20Reference) (Stimulus :type AI%20Stimulus%20Structure))
  (Utilities|Casting|CastToBP_Character_Master Actor)
  (AI|Components|Blackboard|SetValueasBool (AI|GetBlackboard 0) (Utilities|Name|MakeLiteralName "CanChasePlayer") (.bSuccessfullySensed (Utilities|Struct|BreakAIStimulus Stimulus))))

(event OnHPZero(Health)
  (params (DamageType :type Damage%20Type%20Object%20Reference))
  (CallFunction|SetActorFunction false)
  (Development|PrintString (Utilities|GetDisplayName (Components|GetOwner)))
  (Utilities|Casting|CastToBP_MeleeDamageType DamageType
    (:then
      ;[1 1 1] If dead by melee, spawn energy
      (Utilities|FlowControl|Delay 1.2) ; Wait for finishing be strike anim
      (Pawn|Components|CharacterMovement|SetMovementMode (Variables|Character|GetCharacterMovement) "MOVE_Falling" 0))
    (:CastFailed
      (Effects|SpawnEmitteratLocation "/Game/FX/P_ToonExplosion.P_ToonExplosion" (Transformation|GetActorLocation) "0, 0, 0" "3.000000,3.000000,3.000000")
      (Actor|DestroyActor))))

(event EventBeginPlay
  (|CallParentFunction)
  (CallFunction|StartJetpack))

(event Collision|EventActorBeginOverlap
  (params (OtherActor :type Actor%20Object%20Reference)))

(event EventTick
  (params (DeltaSeconds :type Float%20%28single-precision%29)))

(event Game|Damage|EventAnyDamage
  (params (Damage :type Float%20%28single-precision%29) (DamageType :type Damage%20Type%20Object%20Reference) (InstigatedBy :type Controller%20Object%20Reference) (DamageCauser :type Actor%20Object%20Reference))
  (Utilities|Casting|CastToBP_MeleeDamageType DamageType)
  (Development|PrintString "A")
  (if (> (Variables|/Script/TY.HealthComponent|GetHealth (Variables|Default|GetHealth)) 0.0)
    (Development|PrintString "B")
    (CallFunction|SetActorFunction true)
    (else
      (CallFunction|SetActorFunction false))))

(fn ConstructionScript
  (|CallParentFunction))

(fn HandleonHPZero
  (params (NewParam :type Boolean) (DamageType :type Damage%20Type%20Object%20Reference)))

(fn SetActorFunction
  (params (ShouldEnable :type Boolean))
  (bind _self self)
  (bind _returnvalue (AI|GetAIController _self))
  (bind _braincomponent (Variables|/Script/AIModule.AIController|GetBrainComponent _returnvalue))
  (if ShouldEnable
    (Class|BrainComponent|RestartLogic _braincomponent)
    (else
      (AI|Logic|StopLogic _braincomponent "BeStriked")))
  (Class|AIPerceptionComponent|SetSenseEnabled (Variables|Default|GetAIPerception) "/Script/AIModule.AISense" ShouldEnable)
  (Collision|SetActorEnableCollision ShouldEnable)
  (Actor|Tick|SetActorTickEnabled ShouldEnable)
  (Components|Movement|StopMovementImmediately (Variables|Character|GetCharacterMovement)))